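; Sightline actor that visualises a 360-degree line of sight around itself with an instanced static mesh.
; InitialiseISM rebuilds one instance per trace on construction and BeginPlay, then calls SightTrace.
; SightTrace fires evenly spaced, debug-drawn Visibility line traces, rotating and scaling each instance to the hit or range limit.
; BeginPlay also stores the first ClassToFollow actor, though this graph never moves to it or re-traces per tick.
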(event `SightTrace`
  (bind _returnvalue (`self.K2_GetActorLocation`))
  (bind _returnvalue_2 (`KismetMathLibrary.Conv_IntToDouble` (`self.Trace count`)))
  ;[1 1 1] New sight system
  (for _index (range (`self.Trace count`))
    (bind _output_get (set `self.Current trace step` _index))
    (bind (_outhit _returnvalue_3) (`KismetSystemLibrary.LineTraceSingle` :`Start` _returnvalue :`End` (+ _returnvalue (* (`KismetMathLibrary.GreaterGreater_VectorRotator` (`self.GetActorForwardVector`) (`KismetMathLibrary.MakeRotator` 0.0 0.0 (* (`KismetMathLibrary.Conv_IntToDouble` _output_get) (/ 360.0 (`KismetMathLibrary.Conv_IntToDouble` (`self.Trace count`)))))) (`self.check range`))) :`TraceChannel` "TraceTypeQuery1" :`DrawDebugType` "ForDuration" :`DrawTime` 0.1))
    (bind (_bblockinghit _binitialoverlap _time _distance _location _impactpoint _normal _impactnormal _physmat _hitactor _hitcomponent _hitbonename _bonename _hititem _elementindex _faceindex _tracestart _traceend) (`GameplayStatics.BreakHitResult` _outhit))
    (bind _returnvalue_4 (* (`KismetMathLibrary.VSize` (- (`KismetMathLibrary.SelectVector` _location _traceend _returnvalue_3) _tracestart)) (`self.Trace hit offset`)))
    (`InstancedStaticMeshComponent.UpdateInstanceTransform` (`self.InstancedStaticMesh`) (`self.Current trace step`) (`KismetMathLibrary.MakeTransform` (`KismetMathLibrary.SelectVector` (`KismetMathLibrary.MakeVector` 0.0 0.0 (`self.ISM height offset`)) (0.0 0.0 0.0) (`self.Offset by height`)) (`KismetMathLibrary.FindLookAtRotation` _tracestart _traceend) (`KismetMathLibrary.MakeVector` _returnvalue_4 (* (/ 360.0 _returnvalue_2) _returnvalue_2) _returnvalue_4)) false true true)))

(event `Initialise ISM`
  ;[1 1 1] New sight system
  (`InstancedStaticMeshComponent.ClearInstances` (`self.InstancedStaticMesh`))
  (for _ (range (`self.Trace count`))
    (`InstancedStaticMeshComponent.AddInstance` (`self.InstancedStaticMesh`) (`KismetMathLibrary.MakeTransform` (0.0 0.0 0.0)) false))
  (`self.SightTrace`))

(event `self.ReceiveBeginPlay`
  ;[1 1 1] New sight system
  (`|ExecutionSequence`
    (:`then_0`
      (`self.Initialise ISM`)
      (bind _outactors (`GameplayStatics.GetAllActorsOfClass` (`self.Class to follow`)))
      (set `self.Actor to follow` (`|GetArrayItem` _outactors)))))

(fn `UserConstructionScript`
  (`self.Initialise ISM`))